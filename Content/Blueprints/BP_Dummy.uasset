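; BP_Dummy is a character that serves as the victim of a stealth back assassination.
; An overlap sphere shows a tip widget while BP_ThirdPersonCharacter is inside it.
; StealthBackAssassin plays the victim's paired knife montage, starts Ragdoll, hides the tip and returns a reference location and actor rotation for the assassin.
; Ragdoll waits briefly, then enables mesh physics and switches collision profiles, setting the capsule to ignore pawns.
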(event `Ragdoll`
  (`KismetSystemLibrary.Delay` 2.5)
  (`PrimitiveComponent.SetSimulatePhysics` (`self.Mesh`) true)
  (`PrimitiveComponent.SetCollisionProfileName` (`self.CapsuleComponent`) "IgnoreOnlyPawn" true)
  (`PrimitiveComponent.SetCollisionProfileName` (`self.Mesh`) "PhysicsActor" true))

(event `self.AssassinOverlapSphere.OnComponentBeginOverlap`
  (params (OverlappedComponent :type "PrimitiveComponent Object Reference") (OtherActor :type "Actor Object Reference") (OtherComp :type "PrimitiveComponent Object Reference") (OtherBodyIndex :type Integer) (bFromSweep :type Boolean) (SweepResult :type "HitResult Structure (by ref)"))
  (cast `/Game/ThirdPerson/Blueprints/BP_ThirdPersonCharacter` OtherActor)
  (`SceneComponent.SetVisibility` (`self.TipWidget`) true false))

(event `self.AssassinOverlapSphere.OnComponentEndOverlap`
  (params (OverlappedComponent :type "PrimitiveComponent Object Reference") (OtherActor :type "Actor Object Reference") (OtherComp :type "PrimitiveComponent Object Reference") (OtherBodyIndex :type Integer))
  (cast `/Game/ThirdPerson/Blueprints/BP_ThirdPersonCharacter` OtherActor)
  (`SceneComponent.SetVisibility` (`self.TipWidget`) false false))

(fn `StealthBackAssassin`
  (returns (RFLLocation :type "Vector Structure") (AssassinRotation :type "Rotator Structure"))
  (`self.PlayAnimMontage` "/Game/Characters/RPG_Character/Animation/Assassination/Paired_Knife_Stealth_KidneyAndNeck_Vic1_Montage.Paired_Knife_Stealth_KidneyAndNeck_Vic1_Montage")
  (`self.Ragdoll`)
  (`SceneComponent.SetHiddenInGame` (`self.TipWidget`) true false)
  (return (`SceneComponent.K2_GetComponentLocation` (`self.REFLocation`)) (`self.K2_GetActorRotation`)))

(fn `UserConstructionScript`)