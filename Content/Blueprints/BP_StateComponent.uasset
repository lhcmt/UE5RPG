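; BP_StateComponent is a state manager that tracks concurrent movement and action states such as Idle, Jump, Vault and Attack, entering a default state on BeginPlay.
; A data-table row for each requested state defines its relation to every active state: Forbid blocks entry, while Interrupt exits that active state first.
; EnterState and ExitState update the active set, fire enter/exit notifications and print debug output; InterruptState simply wraps ExitState.
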(event `self.ReceiveBeginPlay`
  (`self.EnterState` "NewEnumerator0"))

(fn `CanEnterState`
  (params (StateName :type "/Game/Blueprints/DataType/ENM_State Enum" :default "NewEnumerator0"))
  (returns (bCan :type Boolean) (OutStateToInterrupt :type "Array of /Game/Blueprints/DataType/ENM_State Enum"))
  (locals (StateRelation :type "Map of /Game/Blueprints/DataType/ENM_State Enum to /Game/Blueprints/DataType/ENM_StateRelation Enum") (bCanEnter :type Boolean) (StateToInterrupt :type "Array of /Game/Blueprints/DataType/ENM_State Enum"))
  (bind _staterelation (`local.StateRelation`))
  (bind _returnvalue (`|GetDataTableRow` (`self.StateDataTable`) (`KismetStringLibrary.Conv_StringToName` (`|GetEnumeratorNameAsString` StateName)))
    (:`then`
      (set `local.bCanEnter` true)
      (`|ExecutionSequence`
        (:`then_0`
          (bind (_idle _walk _crouch _jump _climbing _vault _attack) (break `/Game/Blueprints/DataType/STRUCT_PlayerState` _returnvalue))
          (`BlueprintMapLibrary.Map_Add` _staterelation "NewEnumerator0" _idle)
          (`BlueprintMapLibrary.Map_Add` _staterelation "NewEnumerator1" _walk)
          (`BlueprintMapLibrary.Map_Add` _staterelation "NewEnumerator2" _crouch)
          (`BlueprintMapLibrary.Map_Add` _staterelation "NewEnumerator3" _jump)
          (`BlueprintMapLibrary.Map_Add` _staterelation "NewEnumerator4" _climbing)
          (`BlueprintMapLibrary.Map_Add` _staterelation "NewEnumerator5" _vault)
          (`BlueprintMapLibrary.Map_Add` _staterelation "NewEnumerator6" _attack))
        (:`then_1`
          (for _array_element (`self.LocalStateMap`)
            (switch `/Game/Blueprints/DataType/ENM_StateRelation` (`BlueprintMapLibrary.Map_Find` (`local.StateRelation`) _array_element)
              (:`NewEnumerator1`
                (`KismetArrayLibrary.Array_AddUnique` (`local.StateToInterrupt`) _array_element))
              (:`NewEnumerator2`
                (set `local.bCanEnter` false)
                (`KismetSystemLibrary.PrintString` (`KismetStringLibrary.Concat_StrStr` "EnterState :" (`|GetEnumeratorNameAsString` StateName) "Faild , Forbid by:" (`|GetEnumeratorNameAsString` _array_element)))))))
        (:`then_2`
          (return (`local.bCanEnter`) (`local.StateToInterrupt`)))))
    (:`RowNotFound`
      (`KismetSystemLibrary.PrintString` (`KismetStringLibrary.Concat_StrStr` "CantFind State in table :" (`|GetEnumeratorNameAsString` StateName)))
      (return false))))

(fn `EnterState`
  (params (StateName :type "/Game/Blueprints/DataType/ENM_State Enum" :default "NewEnumerator0"))
  (returns (bSuccess :type Boolean))
  (locals (DebugString :type String))
  ;[1 1 1] 已经处于当前状态
  (bind _bhas (`self.HasState` StateName))
  (if _bhas
    (return false)
    (else
      (bind (_bcan _outstatetointerrupt) (`self.CanEnterState` StateName))
      (if _bcan
        (`|ExecutionSequence`
          (:`then_0`
            (for _array_element _outstatetointerrupt
              (`self.ExitState` _array_element)))
          (:`then_1`
            (`KismetArrayLibrary.Array_AddUnique` (`self.LocalStateMap`) StateName)
            (`self.OnStateEnter` StateName)
            (for _array_element_2 (`self.LocalStateMap`)
              (set `local.DebugString` (`KismetStringLibrary.Concat_StrStr` (`local.DebugString`) (`|GetEnumeratorNameAsString` _array_element_2))))
            (`KismetSystemLibrary.PrintString` (`local.DebugString`)))
          (:`then_2`
            (return true)))
        (else
          (return false))))))

(fn `ExitState`
  (params (StateName :type "/Game/Blueprints/DataType/ENM_State Enum" :default "NewEnumerator0"))
  (returns (bSuccess :type Boolean))
  (locals (DebugString :type String))
  (bind _returnvalue (`KismetArrayLibrary.Array_RemoveItem` (`self.LocalStateMap`) StateName))
  (if _returnvalue
    (`self.OnStateExit` StateName)
    (for _array_element (`self.LocalStateMap`)
      (set `local.DebugString` (`KismetStringLibrary.Concat_StrStr` (`local.DebugString`) (`|GetEnumeratorNameAsString` _array_element))))
    (`KismetSystemLibrary.PrintString` (`local.DebugString`))
    (return true)
    (else
      (return false))))

(fn `HasState`
  (params (StateName :type "/Game/Blueprints/DataType/ENM_State Enum" :default "NewEnumerator0"))
  (returns (bHas :type Boolean))
  (return (`KismetArrayLibrary.Array_Contains` (`self.LocalStateMap`) StateName)))

(fn `InterruptState`
  (params (StateName :type "/Game/Blueprints/DataType/ENM_State Enum" :default "NewEnumerator0"))
  (returns (bSuccess :type Boolean))
  (bind _bsuccess (`self.ExitState` StateName))
  (return _bsuccess))