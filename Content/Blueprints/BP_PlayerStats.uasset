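; Player stats component for BP_ThirdPersonCharacter that tracks health and stamina, starting both at their maximums.
; Functions change current values or raise maximums, with some returning depleted, remaining or full status.
; Each change pushes a current-to-max ratio to the UI through the owner's BP_PlayerController.
; IncreaseStamina clamps to MaxHealth rather than MaxStamina, and DecreaseStamina stores its result unclamped.
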(event `self.ReceiveBeginPlay`
  (set `self.CurrentHealth` (`self.MaxHealth`))
  (set `self.CurrentStamina` (`self.MaxStamina`))
  (`self.UpdateHealthPercent`)
  (`self.UpdateStaminaPercent`))

(fn `DecreaseHealth`
  (params (DecreaseHealth :type "Float (double-precision)"))
  (returns (IsDead :type Boolean))
  (bind _output_get (set `self.CurrentHealth` (`KismetMathLibrary.FClamp` (- (`self.CurrentHealth`) DecreaseHealth) 0.0 (`self.MaxHealth`))))
  (`self.UpdateHealthPercent`)
  (bind _returnvalue (<= _output_get 0.0))
  (if _returnvalue
    (return _returnvalue)
    (else
      (return false))))

(fn `DecreaseStamina`
  (params (DecreaseStamina :type "Float (double-precision)"))
  (returns (StaminaLeft :type Boolean))
  (bind _output_get (set `self.CurrentStamina` (- (`self.CurrentStamina`) DecreaseStamina)))
  (`self.UpdateStaminaPercent`)
  (if (<= (`KismetMathLibrary.FClamp` _output_get 0.0 (`self.MaxStamina`)) 0.0)
    (return false)
    (else
      (return true))))

(fn `GetOwnerCharacter`
  (returns (`AsBP Third Person Character` :type "/Game/ThirdPerson/Blueprints/BP_ThirdPersonCharacter Object Reference"))
  (bind _asbp_third_person_character (cast `/Game/ThirdPerson/Blueprints/BP_ThirdPersonCharacter` (`self.GetOwner`)))
  (return _asbp_third_person_character))

(fn `IncreaseMaxHealth`
  (params (IncreaseHealth :type "Float (double-precision)"))
  (set `self.MaxHealth` (+ IncreaseHealth (`self.MaxHealth`)))
  (`self.UpdateHealthPercent`))

(fn `IncreaseMaxStamina`
  (params (IncreaseStamina :type "Float (double-precision)"))
  (set `self.MaxStamina` (+ IncreaseStamina (`self.MaxStamina`)))
  (`self.UpdateStaminaPercent`))

(fn `IncreaseStamina`
  (params (IncreaseStamina :type "Float (double-precision)"))
  (returns (IsFullStamina :type Boolean))
  (set `self.CurrentStamina` (`KismetMathLibrary.FClamp` (+ IncreaseStamina (`self.CurrentStamina`)) 0.0 (`self.MaxHealth`)))
  (`self.UpdateStaminaPercent`)
  (return (>= (`self.CurrentStamina`) (`self.MaxStamina`))))

(fn `UpdateHealthPercent`
  (bind _asbp_player_controller (cast `/Game/Blueprints/BP_PlayerController` (`Pawn.GetController` (`self.GetOwnerCharacter`))))
  (`/Game/Blueprints/BP_PlayerController.UpdateHealthUI` _asbp_player_controller (/ (`self.CurrentHealth`) (`self.MaxHealth`))))

(fn `UpdateStaminaPercent`
  (bind _asbp_player_controller (cast `/Game/Blueprints/BP_PlayerController` (`Pawn.GetController` (`self.GetOwnerCharacter`))))
  (`/Game/Blueprints/BP_PlayerController.UpdateStaminaUI` _asbp_player_controller (/ (`self.CurrentStamina`) (`self.MaxStamina`))))