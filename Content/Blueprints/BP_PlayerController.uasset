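; Player controller that relays health and stamina values to the player's HUD.
; On BeginPlay it casts the HUD to BP_MyHUD and caches the reference.
; UpdateHealthUI and UpdateStaminaUI forward a percent to that HUD's bar updates, skipping the call on dedicated servers.
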(event `self.ReceiveBeginPlay`
  (bind _asbp_my_hud (cast `/Game/UI/BP_MyHUD` (`self.GetHUD`)))
  (set `self.BPMyHUD` _asbp_my_hud))

(fn `UpdateHealthUI`
  (params (Percent :type "Float (double-precision)"))
  (if (not (`KismetSystemLibrary.IsDedicatedServer`))
    (`/Game/UI/BP_MyHUD.UpdateHealthBar` (`self.BPMyHUD`) Percent)))

(fn `UpdateStaminaUI`
  (params (Percent :type "Float (double-precision)"))
  (if (not (`KismetSystemLibrary.IsDedicatedServer`))
    (`/Game/UI/BP_MyHUD.UpdateStamina` (`self.BPMyHUD`) Percent)))

(fn `UserConstructionScript`)